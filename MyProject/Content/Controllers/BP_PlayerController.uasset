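; Player controller that tracks the selected unit in a turn-based, tile grid game and relays orders to it.
; A selection event stores the unit, and an action event forwards the chosen tile to that unit when it is valid.
; Debug keys A and R switch the selected unit's action and advance the turn through its grid.
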(event Custom|Event_UnitSelected
  (params (Unit :type BP%20Unit%20Object%20Reference))
  (Variables|Default|SetSelectedUnit Unit))

(event Custom|Event_DoAction
  (params (SelectedTile :type BP%20Grid%20Tile%20Object%20Reference))
  (bind _selectedunit (Variables|Default|GetSelectedUnit))
  (Utilities|IsValid _selectedunit
    (:Is%20Valid
      (Default|EventDoAction _selectedunit SelectedTile))))

(event Input|KeyboardEvents|R
  (params (Key :type Key%20Structure :default "None"))
  (bind _selectedunit (Variables|Default|GetSelectedUnit))
  ;[1 1 1] DEBUG
  (:Pressed
    (Utilities|IsValid _selectedunit
      (:Is%20Valid
        (Default|EventNextTurn (Variables|/Game/Blueprints/Elements/BP_Element.BP_Element_C|GetGrid _selectedunit))))))

(event Input|KeyboardEvents|A
  (params (Key :type Key%20Structure :default "None"))
  (bind _selectedunit (Variables|Default|GetSelectedUnit))
  ;[1 1 1] DEBUG
  (:Pressed
    (Utilities|IsValid _selectedunit
      (:Is%20Valid
        (Default|EventChangeAction _selectedunit)))))

(fn ConstructionScript)