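; Bp_Obstacle is a grid element that places an obstacle on the level's tile grid.
; The construction script picks a random mesh from its Meshes array and gives it a random yaw in quarter-turn steps for visual variety.
; On BeginPlay, after the parent logic, it registers itself with the Grid at the world location and index from its tile data.
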(event EventBeginPlay
  (bind _value (CallFunction|GetTileData))
  (|CallParentFunction)
  (Default|AddTiletoGrid (Variables|Default|GetGrid) (Utilities|Struct|MakeStruct_Tile (.worldlocation _value) (.gridindex _value) self)))

(fn ConstructionScript
  (bind _meshes (Variables|Default|GetMeshes))
  (bind _staticmesh (Variables|Default|GetStaticMesh))
  (|CallParentFunction)
  (Components|StaticMesh|SetStaticMesh _staticmesh (Utilities|Array|Get(acopy) _meshes (Math|Random|RandomInteger (Utilities|Array|Length _meshes))))
  (Transformation|SetWorldRotation _staticmesh (Math|Rotator|MakeRotator 0.0 0.0 (Math|Conversions|ToFloat(Integer) (* (Math|Random|RandomIntegerinRange 0 3) 90))) false false))