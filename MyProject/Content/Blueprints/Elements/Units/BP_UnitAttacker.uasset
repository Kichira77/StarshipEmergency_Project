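; Attacker unit for a tile-based game, overriding the parent unit's rules for which tiles an action can target or be shown on.
; Move and Attack defer to the parent's checks, while Skill replaces them with an obstacle cast test.
; Skill can be performed only on a tile holding an obstacle, but is also shown on tiles without a valid element.
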(event EventBeginPlay
  (|CallParentFunction) ; This node is disabled and will not be called.\nDrag off pins to build functionality.
)

(event Collision|EventActorBeginOverlap
  (params (OtherActor :type Actor%20Object%20Reference)))

(event EventTick
  (params (DeltaSeconds :type Float%20%28single-precision%29)))

(fn ConstructionScript
  (|CallParentFunction))

(fn CanDoActiononTile
  (params (SelectedTile :type BP%20Grid%20Tile%20Object%20Reference))
  (bind _condition (|CallParentFunction SelectedTile))
  (switch Utilities|FlowControl|Switch|SwitchonEnum_UnitAction (Variables|Default|GetAction)
    (:NewEnumerator1
      _)
    (:NewEnumerator0
      _)
    (:NewEnumerator3
      (return (.bSuccess (Utilities|Casting|CastToBp_Obstacle (.element (Default|GetTileData SelectedTile)))))))
  (return _condition))

(fn CanShowActiononTile
  (params (Element :type BP%20Element%20Object%20Reference))
  (bind _condition (|CallParentFunction Element))
  (switch Utilities|FlowControl|Switch|SwitchonEnum_UnitAction (Variables|Default|GetAction)
    (:NewEnumerator1
      _)
    (:NewEnumerator0
      _)
    (:NewEnumerator3
      (return (or (.bSuccess (Utilities|Casting|CastToBp_Obstacle Element)) (not (Utilities|IsValid Element))))))
  (return _condition))