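; BP_Element is an actor that occupies a tile on the BP_Grid and registers itself in that tile's data.
; One tick after BeginPlay it scans all grid tiles for the nearest, snaps to it with a downward Z offset, and writes itself into the Tiles map.
; SetNewPosition clears the old tile's element and claims the grid's selected tile, updating only the data, not the actor's location.
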(event EventBeginPlay
  (bind _outactors (Actor|GetAllActorsOfClass "/Game/Blueprints/Grid/BP_Grid.BP_Grid_C"))
  (Variables|Grid|SetGrid (Utilities|Array|Get(acopy) _outactors))
  (Utilities|FlowControl|DelayUntilNextTick)
  (CallFunction|SetGridIndexandSnaptoLocation))

(fn ConstructionScript)

(fn SetGridIndexandSnaptoLocation
  (bind _grid (Variables|Grid|GetGrid))
  (bind _tiles (Variables|/Game/Blueprints/Grid/BP_Grid.BP_Grid_C|GetTiles _grid))
  (LocalVariables|SetClosestDistance 9999999999.0)
  (bind _keys (Utilities|Map|Keys (Variables|/Game/Blueprints/Grid/BP_Grid.BP_Grid_C|GetTiles (Variables|Grid|GetGrid))))
  (for _array_element _keys
    (if (< (Math|Vector|VectorLength (- (.worldlocation (.Value (Utilities|Map|Find (Variables|/Game/Blueprints/Grid/BP_Grid.BP_Grid_C|GetTiles (Variables|Grid|GetGrid)) _array_element))) (Transformation|GetActorLocation self))) (LocalVariables|GetClosestDistance))
      (LocalVariables|SetClosestDistance (Math|Vector|VectorLength (- (.worldlocation (.Value (Utilities|Map|Find (Variables|/Game/Blueprints/Grid/BP_Grid.BP_Grid_C|GetTiles (Variables|Grid|GetGrid)) _array_element))) (Transformation|GetActorLocation self))))
      (LocalVariables|SetClosestIndex (.gridindex (.Value (Utilities|Map|Find (Variables|/Game/Blueprints/Grid/BP_Grid.BP_Grid_C|GetTiles (Variables|Grid|GetGrid)) _array_element))))))
  (Variables|Grid|SetGridIndex (LocalVariables|GetClosestIndex))
  (Transformation|SetActorLocation (Math|Vector|MakeVector (.x (.worldlocation (.Value (Utilities|Map|Find _tiles (LocalVariables|GetClosestIndex))))) (.y (.worldlocation (.Value (Utilities|Map|Find _tiles (LocalVariables|GetClosestIndex))))) (- (.z (.worldlocation (.Value (Utilities|Map|Find _tiles (LocalVariables|GetClosestIndex))))) 4e+01)) false false)
  (Utilities|Map|Add _tiles (.gridindex (.Value (Utilities|Map|Find _tiles (LocalVariables|GetClosestIndex)))) (Utilities|Struct|MakeStruct_Tile (Math|Vector|MakeVector (.x (.worldlocation (.Value (Utilities|Map|Find _tiles (LocalVariables|GetClosestIndex))))) (.y (.worldlocation (.Value (Utilities|Map|Find _tiles (LocalVariables|GetClosestIndex))))) (.z (.worldlocation (.Value (Utilities|Map|Find _tiles (LocalVariables|GetClosestIndex)))))) (.gridindex (.Value (Utilities|Map|Find _tiles (LocalVariables|GetClosestIndex)))) self)))

(fn SetTileElement
  (params (Element :type BP%20Element%20Object%20Reference))
  (bind _grid (Variables|Grid|GetGrid))
  (bind _gridindex (Variables|Grid|GetGridIndex))
  (bind _tiles (Variables|/Game/Blueprints/Grid/BP_Grid.BP_Grid_C|GetTiles _grid))
  (bind _value (Utilities|Map|Find _tiles _gridindex))
  (Utilities|Map|Add _tiles _gridindex (Utilities|Struct|MakeStruct_Tile (.worldlocation _value) (.gridindex _value) Element)))

(fn SetNewPosition
  (CallFunction|SetTileElement)
  (Variables|Grid|SetGridIndex (Variables|/Game/Blueprints/Grid/BP_GridTile.BP_GridTile_C|GetGridIndex (Variables|/Game/Blueprints/Grid/BP_Grid.BP_Grid_C|GetSelectedTile (Variables|Grid|GetGrid))))
  (CallFunction|SetTileElement self))

(fn GetTileData
  (return (.Value (Utilities|Map|Find (Variables|/Game/Blueprints/Grid/BP_Grid.BP_Grid_C|GetTiles (Variables|Grid|GetGrid)) (Variables|Grid|GetGridIndex)))))