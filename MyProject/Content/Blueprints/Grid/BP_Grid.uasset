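; Tactical grid manager for a turn-based, team-based unit game, holding tile data and turn, energy and combat rules.
; BeginPlay builds an index-keyed tile map, scatters random obstacles, spawns tile actors and starts the turn; the construction script previews the grid with debug drawing.
; Selected units' relative move, attack or skill patterns become bounds-checked hover tiles.
; Turn changes refill energy, clear highlights and attempt respawns of dead units.
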(event Custom|Event_ShowPattern
  (params (SelectedUnit :type BP%20Unit%20Object%20Reference))
  (Pattern|GeneratePattern SelectedUnit))

(event Custom|Event_TileClicked
  (params (TileIndex :type Vector%202D%20Structure))
  (bind _output_get (Variables|Grid|SetSelectedTile (.Value (Utilities|Map|Find (Variables|Grid|GetGridTiles) TileIndex))))
  (Default|EventDoAction (Variables|Default|GetPlayerController) _output_get))

(event Custom|Event_NextTurn
  (if (Game|IsFirstTurn)
    ;[1 1 1] Ajoute un tour joué
    (Math|Integer|IncrementInt (Variables|Game|GetCurrentTurn)
      (:%20%20
        _))
    (else
      ;[1 1 1] Change l'équipe courante
      (bind _result (Math|Integer|IncrementInt (Math|Conversions|ToInteger(Byte) (Variables|Game|GetTeamTurn)))
        (:%20%20
          (Variables|Game|SetTeamTurn (Utilities|Enum|ByteToEnumEnum_UnitTeam (Math|Conversions|ToByte(Integer) (Math|Integer|%(Integer) _result (|GetNumEnumEntries)))))))))
  ;[1 1 1] Réinitialisation de l'énergie
  (Variables|Game|SetCurrentEnergy (Variables|Game|GetEnergyByTurn))
  (Default|EventUnitSelected (Variables|Default|GetPlayerController))
  (Pattern|ClearPattern)
  (Game|TryRespawnDeadUnits)
  ;[1 1 1] DEBUG
  (Development|PrintString (Utilities|String|Append (Utilities|String|EnumtoString (Variables|Game|GetTeamTurn)) " turn")))

(event EventBeginPlay
  (bind _returnvalue (Game|GetPlayerController 0))
  (Variables|/Script/Engine.PlayerController|SetbShowMouseCursor _returnvalue true)
  (Variables|/Script/Engine.PlayerController|SetbEnableMouseOverEvents _returnvalue true)
  (Rendering|Debug|FlushPersistentDebugLines)
  (Variables|Grid|SetGridLocation (Transformation|GetWorldLocation (Variables|Default|GetScene)))
  (Grid|GenerateMapDatafromWorld)
  (Grid|GenerateObstacles)
  (Grid|SpawnTiles)
  (Variables|Default|SetPlayerController (.AsBP%20Player%20Controller (Utilities|Casting|CastToBP_PlayerController (Game|GetPlayerController 0))))
  (CallFunction|EventNextTurn))

(fn ConstructionScript
  (bind _gridsizeworld (Variables|Grid|GetGridSizeWorld))
  (Rendering|Debug|FlushPersistentDebugLines)
  (Variables|Grid|SetGridLocation (Transformation|GetWorldLocation (Variables|Default|GetScene)))
  ;[1 1 1] Contour de la grille
  (Rendering|Debug|DrawDebugBox (Variables|Grid|GetGridLocation) (Math|Vector|MakeVector (.y _gridsizeworld) (.x _gridsizeworld) 5.0) "(R=0.000000,G=0.004940,B=1.000000,A=1.000000)" "0, 0, 0" 1e+09 1e+01)
  (Grid|GenerateMapDatafromWorld)
  (Debug|DrawTile))

(fn GridBottomLeft
  (return (- (- (Variables|Grid|GetGridLocation) (* (Math|Vector|GetRightVector (Variables|Default|GetScene)) (.x (Variables|Grid|GetGridSizeWorld)))) (* (Math|Vector|GetForwardVector (Variables|Default|GetScene)) (.y (Variables|Grid|GetGridSizeWorld))))))

(fn MySphereTrace
  (params (Start :type Vector) (TraceChannel :type ETraceTypeQuery%20Enum :default "TraceTypeQuery1"))
  (bind (_outhit _returnvalue) (Collision|SphereTraceByChannel Start Start (- (Variables|Grid|GetTileSize) (Variables|Grid|GetTileSizeMinus)) TraceChannel false 0 "None" true "(R=1.000000,G=0.000000,B=0.000000,A=1.000000)" "(R=0.000000,G=1.000000,B=0.000000,A=1.000000)" 2e+01))
  (return _returnvalue (.hitactor _outhit)))

(fn GridTileNumber
  (bind _gridsizeworld (Variables|Grid|GetGridSizeWorld))
  (bind _tilesize (Variables|Grid|GetTileSize))
  (bind _returnvalue (/ _gridsizeworld (Math|Vector2D|MakeVector2D _tilesize _tilesize)))
  (return (- (Math|Float|Round (.x _returnvalue)) 1) (- (Math|Float|Round (.y _returnvalue)) 1)))

(fn GenerateMapDatafromWorld
  (bind (_idtilenumberx _idtilenumbery) (Grid|GridTileNumber))
  (for _index (range 0 _idtilenumberx)
    (LocalVariables|Setx _index)
    (for _index_2 (range 0 _idtilenumbery)
      (LocalVariables|Sety _index_2)
      (LocalVariables|SetTilePosition (+ (Grid|GridBottomLeft) (Utilities|GetPositionX (LocalVariables|Getx)) (Utilities|GetPositionY (LocalVariables|Gety))))
      (Grid|AddTiletoGrid (Utilities|Struct|MakeStruct_Tile (LocalVariables|GetTilePosition) (Math|Vector2D|MakeVector2D (Math|Conversions|ToFloat(Integer) (LocalVariables|Getx)) (Math|Conversions|ToFloat(Integer) (LocalVariables|Gety))) 0)))))

(fn DrawTile
  (bind _tiles (Variables|Grid|GetTiles))
  (bind _keys (Utilities|Map|Keys _tiles))
  (for _array_element _keys
    (Debug|MyDrawDebugPlane (.worldlocation (.Value (Utilities|Map|Find _tiles _array_element))))))

(fn MyDrawDebugPlane
  (params (Location :type Vector))
  (Class|KismetSystemLibrary|DrawDebugPlane (Utilities|Struct|MakePlane (.Z (Class|KismetMathLibrary|BreakVector3f Location)) 0.0 0.0 1.0) Location (- (Variables|Grid|GetTileSize) (* (Variables|Grid|GetTileSize) 0.05)) "(R=1.000000,G=1.000000,B=1.000000,A=0.019608)" 1e+07))

(fn AddTiletoGrid
  (params (TileData :type Struct%20Tile%20Structure))
  (Utilities|Map|Add (Variables|Grid|GetTiles) (.gridindex TileData) (Utilities|Struct|MakeStruct_Tile (.worldlocation TileData) (.gridindex TileData) (.element TileData))))

(fn SpawnTiles
  (bind _tiles (Variables|Grid|GetTiles))
  (bind _keys (Utilities|Map|Keys _tiles))
  (for _array_element _keys
    (bind _returnvalue (Game|SpawnActorfromClass "/Game/Blueprints/Grid/BP_GridTile.BP_GridTile_C" (Math|Conversions|ToTransform(Vector) (- (.worldlocation (.Value (Utilities|Map|Find _tiles _array_element))) "0,0.000000,250.000000")) "Undefined" 0 0))
    (Variables|/Game/Blueprints/Grid/BP_GridTile.BP_GridTile_C|SetGridIndex _returnvalue _array_element)
    (Variables|/Game/Blueprints/Grid/BP_GridTile.BP_GridTile_C|SetGrid _returnvalue self)
    (Utilities|Map|Add (Variables|Grid|GetGridTiles) _array_element _returnvalue)))

(fn GeneratePattern
  (params (SelectedUnit :type BP%20Unit%20Object%20Reference))
  (Pattern|ClearPattern)
  (Pattern|SetPatternbyAction)
  (for _array_element (Variables|Pattern|GetPattern)
    (bind _condition (Default|CanShowActiononTile SelectedUnit (.element (.Value (Utilities|Map|Find (Variables|Grid|GetTiles) _array_element)))))
    (if _condition
      (bind _returnvalue (Game|SpawnActorfromClass "/Game/Blueprints/Grid/BP_TileHover.BP_TileHover_C" (Math|Transform|MakeTransform (.worldlocation (.Value (Utilities|Map|Find (Variables|Grid|GetTiles) _array_element))) "0, 0, 0" "1.000000,1.000000,1.000000") "Undefined" 0 0))
      (Variables|/Game/Blueprints/Grid/BP_TileHover.BP_TileHover_C|SetTileIndex _returnvalue _array_element)
      (Variables|/Game/Blueprints/Grid/BP_TileHover.BP_TileHover_C|SetGrid _returnvalue self)
      (Pattern|ColorPatternbyAction)))
  (return))

(fn SetPatternbyAction
  (bind _playercontroller (Variables|Default|GetPlayerController))
  (bind _selectedunit (Variables|/Game/Controllers/BP_PlayerController.BP_PlayerController_C|GetSelectedUnit _playercontroller))
  (switch Utilities|FlowControl|Switch|SwitchonEnum_UnitAction (Variables|/Game/Blueprints/Elements/Units/BP_Unit.BP_Unit_C|GetAction _selectedunit)
    (:NewEnumerator1
      (bind _absolutepattern (Pattern|ConvertPattern (Variables|/Game/Blueprints/Elements/Units/BP_Unit.BP_Unit_C|GetMovePattern _selectedunit)))
      (Variables|Pattern|SetPattern _absolutepattern))
    (:NewEnumerator0
      (bind _keys (Utilities|Map|Keys (Variables|/Game/Blueprints/Elements/Units/BP_Unit.BP_Unit_C|GetAttackPattern _selectedunit)))
      (bind _absolutepattern_2 (Pattern|ConvertPattern _keys))
      (Variables|Pattern|SetPattern _absolutepattern_2))
    (:NewEnumerator3
      (bind _absolutepattern_3 (Pattern|ConvertPattern (Variables|/Game/Blueprints/Elements/Units/BP_Unit.BP_Unit_C|GetSkillPattern _selectedunit)))
      (Variables|Pattern|SetPattern _absolutepattern_3)))
  (return))

(fn ColorPatternbyAction
  (bind _outactors (Actor|GetAllActorsOfClass "/Game/Blueprints/Grid/BP_TileHover.BP_TileHover_C"))
  (for _array_element _outactors
    (Default|EventSetAction _array_element (Variables|/Game/Controllers/BP_PlayerController.BP_PlayerController_C|GetSelectedUnit (Variables|Default|GetPlayerController))))
  (return))

(fn ClearPattern
  (bind _outactors (Actor|GetAllActorsOfClass "/Game/Blueprints/Grid/BP_TileHover.BP_TileHover_C"))
  (for _array_element _outactors
    (Actor|DestroyActor _array_element))
  (return))

(fn ConvertPattern
  (params (RelativePattern :type Array%20of%20Vector%202D%20Structures))
  (bind (_idtilenumberx _idtilenumbery) (Grid|GridTileNumber))
  (for _array_element RelativePattern
    (if (Math|Boolean|ANDBoolean (>= (.x (+ _array_element (Variables|/Game/Blueprints/Elements/BP_Element.BP_Element_C|GetGridIndex (Variables|/Game/Controllers/BP_PlayerController.BP_PlayerController_C|GetSelectedUnit (Variables|Default|GetPlayerController))))) 0.0) (>= (.y (+ _array_element (Variables|/Game/Blueprints/Elements/BP_Element.BP_Element_C|GetGridIndex (Variables|/Game/Controllers/BP_PlayerController.BP_PlayerController_C|GetSelectedUnit (Variables|Default|GetPlayerController))))) 0.0) (<= (.x (+ _array_element (Variables|/Game/Blueprints/Elements/BP_Element.BP_Element_C|GetGridIndex (Variables|/Game/Controllers/BP_PlayerController.BP_PlayerController_C|GetSelectedUnit (Variables|Default|GetPlayerController))))) _idtilenumberx) (<= (.y (+ _array_element (Variables|/Game/Blueprints/Elements/BP_Element.BP_Element_C|GetGridIndex (Variables|/Game/Controllers/BP_PlayerController.BP_PlayerController_C|GetSelectedUnit (Variables|Default|GetPlayerController))))) _idtilenumbery))
      (Utilities|Array|Add (LocalVariables|GetPatternL) (Math|Vector2D|MakeVector2D (.x (+ _array_element (Variables|/Game/Blueprints/Elements/BP_Element.BP_Element_C|GetGridIndex (Variables|/Game/Controllers/BP_PlayerController.BP_PlayerController_C|GetSelectedUnit (Variables|Default|GetPlayerController))))) (.y (+ _array_element (Variables|/Game/Blueprints/Elements/BP_Element.BP_Element_C|GetGridIndex (Variables|/Game/Controllers/BP_PlayerController.BP_PlayerController_C|GetSelectedUnit (Variables|Default|GetPlayerController)))))))))
  (return (LocalVariables|GetPatternL)))

(fn GetRandomGridIndex
  (bind (_idtilenumberx _idtilenumbery) (Grid|GridTileNumber))
  (return (Math|Vector2D|MakeVector2D (Math|Conversions|ToFloat(Integer) (Math|Random|RandomIntegerinRange 0 _idtilenumberx)) (Math|Conversions|ToFloat(Integer) (Math|Random|RandomIntegerinRange 0 _idtilenumbery)))))

(fn GenerateObstacles
  (while (< (LocalVariables|GetObstaclesDefined) (Variables|Grid|GetTotalObstacles))
    (bind _index (Grid|GetRandomGridIndex))
    (if (and (not (Utilities|Array|ContainsItem (Variables|Grid|GetObstacleCannotSpawn) _index)) (not (Utilities|IsValid (.element (.Value (Utilities|Map|Find (Variables|Grid|GetTiles) _index))))))
      (Math|Integer|IncrementInt (LocalVariables|GetObstaclesDefined)
        (:%20%20
          (bind _returnvalue (Game|SpawnActorfromClass "/Game/Blueprints/Elements/Bp_Obstacle.Bp_Obstacle_C" (Math|Transform|MakeTransform (+ (Utilities|GetPositionX (Math|Float|Truncate (.X (Math|Vector2D|BreakVector2D _index)))) (Utilities|GetPositionY (Math|Float|Truncate (.Y (Math|Vector2D|BreakVector2D _index)))) (Grid|GridBottomLeft)) "0, 0, 0" "1.000000,1.000000,1.000000") "Undefined" 0 0))
          (Grid|AddTiletoGrid (Utilities|Struct|MakeStruct_Tile (+ (Utilities|GetPositionX (Math|Float|Truncate (.X (Math|Vector2D|BreakVector2D _index)))) (Utilities|GetPositionY (Math|Float|Truncate (.Y (Math|Vector2D|BreakVector2D _index)))) (Grid|GridBottomLeft)) (Math|Vector2D|MakeVector2D (.X (Math|Vector2D|BreakVector2D _index)) (.Y (Math|Vector2D|BreakVector2D _index))) _returnvalue))))))
  (return))

(fn DebugPrintAllElements
  (bind _tiles (Variables|Grid|GetTiles))
  (bind _tiles_2 (Variables|Grid|GetTiles))
  (bind _value (Utilities|Map|Find _tiles_2 "(X=6.000000,Y=7.000000)"))
  (bind _keys (Utilities|Map|Keys _tiles))
  (for _array_element _keys
    (Utilities|IsValid (.element (.Value (Utilities|Map|Find _tiles _array_element)))
      (:Is%20Valid
        (Utilities|Casting|CastToBP_Unit (.element (.Value (Utilities|Map|Find _tiles _array_element))))
        (Development|PrintString (Utilities|String|Append "el: " (Utilities|String|ToString(Vector2d) (.gridindex (.Value (Utilities|Map|Find _tiles _array_element)))) ", " (Utilities|GetDisplayName (.element (.Value (Utilities|Map|Find _tiles _array_element))))) true true "(R=0.000000,G=0.660000,B=1.000000,A=1.000000)" 535424.0)
        (Development|PrintString (Utilities|String|Append (Utilities|String|ToString(Vector) (.worldlocation _value)) ", " (Utilities|String|ToString(Vector2d) (.gridindex _value)) ", " (Utilities|GetDisplayName (.element _value))) true true "(R=0.000000,G=0.660000,B=1.000000,A=1.000000)" 2.25205025e+09)))))

(fn IsPlayerTurn
  (params (Unit :type BP%20Unit%20Object%20Reference))
  (return (Utilities|Enum|Equal(Enum) (Variables|/Game/Blueprints/Elements/Units/BP_Unit.BP_Unit_C|GetTeam Unit) (Variables|Game|GetTeamTurn))))

(fn GetEnergyCost
  (params (Action :type Enum_UnitAction%20Enum :default "NewEnumerator1"))
  (switch Utilities|FlowControl|Switch|SwitchonEnum_UnitAction Action
    (:NewEnumerator1
      (return 1))
    (:NewEnumerator0
      (return 2))
    (:NewEnumerator3
      (return 2))))

(fn GetAttackDamage
  (params (Attack :type Enum_UnitAttackDamage%20Enum :default "NewEnumerator0"))
  (switch Utilities|FlowControl|Switch|SwitchonEnum_UnitAttackDamage Attack
    (:NewEnumerator0
      (return 4))
    (:NewEnumerator1
      (return 3))
    (:NewEnumerator2
      (return 2))))

(fn CanSelectUnit
  (params (Unit :type BP%20Unit%20Object%20Reference))
  (bind _isplayerturn (Game|IsPlayerTurn Unit))
  (return _isplayerturn))

(fn IsFirstTurn
  (return (== (Variables|Game|GetCurrentTurn) 0)))

(fn KillUnit
  (params (Unit :type BP%20Unit%20Object%20Reference))
  (bind _value (Default|GetTileData Unit))
  (Default|SetTileElement Unit)
  (Variables|/Game/Blueprints/Elements/Units/BP_Unit.BP_Unit_C|SetTurnRespawn Unit (Variables|Game|GetRespawnTurn))
  (Variables|/Game/Blueprints/Elements/Units/BP_Unit.BP_Unit_C|SetIsDead Unit true)
  (Transformation|SetActorLocation Unit (Math|Vector|MakeVector (.x (.worldlocation _value)) (.y (.worldlocation _value)) -1e+03) false false))

(fn TryRespawnDeadUnits
  (bind _outactors (Actor|GetAllActorsOfClass "/Game/Blueprints/Elements/Units/BP_Unit.BP_Unit_C"))
  (for _array_element _outactors
    (Default|TryRespawn _array_element)))