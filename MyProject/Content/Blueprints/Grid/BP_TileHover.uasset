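; BP_TileHover is a grid tile highlight whose plane shows the acting unit's current action and reports clicks to the grid.
; Event_SetAction tints the plane's Action material parameter by action type: Move, Attack or Skill.
; For attacks, the tile's offset from the unit is looked up in the unit's AttackPattern to pick a heavy, normal or light color.
; Clicking the plane passes the tile index to the Grid.
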(event OnClicked(Plane)
  (params (TouchedComponent :type Primitive%20Component%20Object%20Reference) (ButtonPressed :type Key%20Structure))
  (Default|EventTileClicked (Variables|Tile|GetGrid) (Variables|Tile|GetTileIndex)))

(event Custom|Event_SetAction
  (params (Unit :type BP%20Unit%20Object%20Reference))
  (switch Utilities|FlowControl|Switch|SwitchonEnum_UnitAction (Variables|/Game/Blueprints/Elements/Units/BP_Unit.BP_Unit_C|GetAction Unit)
    (:NewEnumerator1
      (Rendering|Material|SetVectorParameterValueonMaterials (Variables|Default|GetPlane) "Action" (Math|Conversions|ToVector(LinearColor) (Variables|Default|GetMoveColor))))
    (:NewEnumerator0
      (switch Utilities|FlowControl|Switch|SwitchonEnum_UnitAttackDamage (.Value (Utilities|Map|Find (Variables|/Game/Blueprints/Elements/Units/BP_Unit.BP_Unit_C|GetAttackPattern Unit) (- (Variables|Tile|GetTileIndex) (Variables|/Game/Blueprints/Elements/BP_Element.BP_Element_C|GetGridIndex Unit))))
        (:NewEnumerator0
          (Variables|Default|SetAttackColor (Variables|Default|GetAttackColorHeavy)))
        (:NewEnumerator1
          (Variables|Default|SetAttackColor (Variables|Default|GetAttackColorNormal)))
        (:NewEnumerator2
          (Variables|Default|SetAttackColor (Variables|Default|GetAttackColorLight))))
      (Rendering|Material|SetVectorParameterValueonMaterials (Variables|Default|GetPlane) "Action" (Math|Conversions|ToVector(LinearColor) (Variables|Default|GetAttackColor))))
    (:NewEnumerator3
      (Rendering|Material|SetVectorParameterValueonMaterials (Variables|Default|GetPlane) "Action" (Math|Conversions|ToVector(LinearColor) (Variables|Default|GetSkillColor))))))

(fn ConstructionScript)