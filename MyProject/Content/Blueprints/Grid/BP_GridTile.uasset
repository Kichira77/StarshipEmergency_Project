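; BP_GridTile is a grid tile actor that picks a random mesh on construction and reports clicks to its Grid.
; It reads its data from the Grid's Tiles map by GridIndex.
; Shortly after BeginPlay, obstacle tiles spawn Bp_Obstacle below the tile location and write that actor back into the map.
; Cursor events only set IsHovered, as the function spawning or destroying BP_TileHover is never called here.
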(event Custom|Event_DeselectedTile)

(event EventBeginPlay
  (Utilities|FlowControl|Delay 0.1)
  (CallFunction|SetTileObstacle))

(event MouseInput|EventActorBeginCursorOver
  (Variables|Tile|SetIsHovered true))

(event MouseInput|EventActorEndCursorOver
  (Variables|Tile|SetIsHovered false))

(event MouseInput|EventActorOnClicked
  (params (ButtonPressed :type Key%20Structure))
  (Default|EventTileClicked (Variables|Tile|GetGrid) self))

(fn ConstructionScript
  (bind _meshes (Variables|Mesh|GetMeshes))
  (Components|StaticMesh|SetStaticMesh (Variables|Default|GetStaticMesh) (Utilities|Array|Get(acopy) _meshes (Math|Random|RandomInteger (Utilities|Array|Length _meshes)))))

(fn GetTileData
  (return (.Value (Utilities|Map|Find (Variables|/Game/Blueprints/Grid/BP_Grid.BP_Grid_C|GetTiles (Variables|Tile|GetGrid)) (Variables|Tile|GetGridIndex)))))

(fn SetTileObstacle
  (bind _value (CallFunction|GetTileData))
  (bind _grid (Variables|Tile|GetGrid))
  (bind _gridindex (Variables|Tile|GetGridIndex))
  (bind _tiles (Variables|/Game/Blueprints/Grid/BP_Grid.BP_Grid_C|GetTiles _grid))
  (bind _value_2 (Utilities|Map|Find _tiles _gridindex))
  (switch Utilities|FlowControl|Switch|SwitchonEnum_TileTypes (.tiletype _value)
    (:NewEnumerator3
      (bind _returnvalue (Game|SpawnActorfromClass "/Game/Blueprints/Elements/Bp_Obstacle.Bp_Obstacle_C" (Math|Conversions|ToTransform(Vector) (- (.worldlocation _value) "0,0,80.000000")) "Undefined" 0 0))
      (Utilities|Map|Add _tiles _gridindex (Utilities|Struct|MakeStruct_Tile (.tiletype _value_2) (.worldlocation _value_2) (.gridindex _value_2) _returnvalue)))))

(fn SetTileHover
  (bind _value (CallFunction|GetTileData))
  (if (Variables|Tile|GetIsHovered)
    (if (not (Utilities|Enum|Equal(Enum) (.tiletype _value) "NewEnumerator3"))
      (bind _returnvalue (Game|SpawnActorfromClass "/Game/Blueprints/Grid/BP_TileHover.BP_TileHover_C" (Math|Conversions|ToTransform(Vector) (- (.worldlocation _value) "0,0,25.000000")) "Undefined" 0 0))
      (Variables|Tile|SetTileHover _returnvalue))
    (elif (Utilities|IsValid (Variables|Tile|GetTileHover))
      (Actor|DestroyActor (Variables|Tile|GetTileHover)))))